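; BP_SWAIController is an AI controller for test enemies that starts their behavior tree and tracks the player.
; BeginPlay sets up the blackboard and runs the behavior tree.
; Perception updates write a successfully sensed BP_Player_Test into the "Player" blackboard key, which is not cleared when sensing fails.
; A disconnected, unfinished snippet would set "TargetDistance" to zero but never runs.
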(event OnTargetPerceptionUpdated(AIPerception)
  (params (Actor :type Actor%20Object%20Reference) (Stimulus :type AI%20Stimulus%20Structure))
  (bind _asbp_player_test (Utilities|Casting|CastToBP_Player_Test Actor))
  (if (.bSuccessfullySensed (Utilities|Struct|BreakAIStimulus Stimulus))
    (AI|Components|Blackboard|SetValueasObject (AI|GetBlackboard 0) (Utilities|Name|MakeLiteralName "Player") _asbp_player_test)))

(event EventBeginPlay
  (Class|AIController|UseBlackboard (Variables|Default|GetBlackboard%20Asset))
  (AI|RunBehaviorTree (Variables|Default|GetBTAsset)))

(event EventTick
  (params (DeltaSeconds :type Float%20%28single-precision%29)))

(fn ConstructionScript)