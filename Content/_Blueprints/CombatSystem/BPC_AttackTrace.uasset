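; Combat component that detects melee weapon hits by sweeping traces along a single registered weapon mesh during an attack.
; While tracing, a fast looping timer samples points between two weapon sockets and box-traces from each point's previous position to its current one, covering the swing between ticks.
; Each newly hit actor fires the attack-hit event once per attack; ending the trace stops the timer and clears the hit list.
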(event Custom|Start%20Attack%20Trace
  ;[1 1 1] 开启攻击检测
  (Variables|Default|SetBox%20Height (CallFunction|GetBoxHeight))
  (CallFunction|UpdateCheckPointLocation)
  (bind _returnvalue (Utilities|Time|SetTimerbyEvent (delegate Custom|On%20Attack%20Trace) 0.01 true)))

(event Custom|On%20Attack%20Trace
  (bind _check_points (Variables|Default|GetCheck%20Points))
  (if (Variables|参数|GetShould%20Check?)
    (bind _pre_check_points (CallFunction|UpdateCheckPointLocation))
    (for (_ _array_index) _check_points
      (bind _outhits (Class|KismetSystemLibrary|BoxTraceMultiforObjects (Utilities|Array|Get(acopy) _pre_check_points _array_index) (Utilities|Array|Get(acopy) _check_points _array_index) (Math|Vector|MakeVector 2e+01 (* (/ (Variables|Default|GetBox%20Height) (Variables|Parameter|GetCheck%20Point%20Num)) 2.0) 2e+01) (Math|Rotator|FindLookatRotation (Utilities|Array|Get(acopy) _pre_check_points _array_index) (Utilities|Array|Get(acopy) _check_points _array_index)) (Variables|Parameter|GetObject%20Types) false (Variables|Parameter|GetActors%20to%20Ignore) "ForDuration" true "(R=1.000000,G=0.000000,B=0.000000,A=1.000000)" "(R=0.000000,G=1.000000,B=0.000000,A=1.000000)" 0.2))
      (for _array_element _outhits
        (bind _output_get (Variables|Default|SetLast%20Hit _array_element))
        ;[1 1 1] 如果对象已经被击中过，在结束攻击之前不会再次被击中
        (if (not (Utilities|Array|ContainsItem (Variables|Default|GetAlready%20Hit%20Actor) (.HitActor (Collision|BreakHitResult _output_get))))
          (bind _output_get_2 (Variables|Default|SetHit%20Actor (.HitActor (Collision|BreakHitResult _output_get))))
          (Utilities|Array|Add (Variables|Default|GetAlready%20Hit%20Actor) _output_get_2)
          (Default|CallOnAttackHitEvent (Variables|Default|GetLast%20Hit) false))))))

(event Custom|End%20Attack%20Trace
  ;[1 1 1] 关闭攻击检测
  (Utilities|Time|ClearandInvalidateTimerbyHandle (stale Custom|Start%20Attack%20Trace _returnvalue))
  ;;[1 1 1] 清空上一轮攻击的命中结果
  (Utilities|Array|Clear (Variables|Default|GetAlready%20Hit%20Actor)))

(event EventBeginPlay
  (bind _ascharacter (Utilities|Casting|CastToCharacter (Components|GetOwner)))
  (Variables|OwnerInfo|SetOwner _ascharacter))

(fn AddTraceMesh
  (params (Trace%20Mesh :type Primitive%20Component%20Object%20Reference))
  ;[1 1 1] 之后考虑升级成可以加入多个武器的
  (Variables|Default|SetWeapons Trace%20Mesh))

(fn UpdateCheckPointLocation
  (bind _weapons (Variables|Default|GetWeapons))
  (bind _end_socket_name (Variables|Parameter|GetEnd%20Socket%20Name))
  (bind _returnvalue (Transformation|GetSocketTransform _weapons _end_socket_name "RTS_World"))
  (Utilities|FlowControl|Sequence
    (:then_0
      ;[1 1 1] 保存之前的向量&清空
      (LocalVariables|SetPre%20Check%20Point (Variables|Default|GetCheck%20Points))
      (Utilities|Array|Clear (Variables|Default|GetCheck%20Points)))
    (:then_1
      (for _index (range 0 (Variables|Parameter|GetCheck%20Point%20Num))
        (Utilities|Array|Add (Variables|Default|GetCheck%20Points) (+ (* _index (/ (- (.location (Transformation|GetSocketTransform (Variables|Default|GetWeapons) (Variables|Parameter|GetStart%20Socket%20Name) "RTS_World")) (.location _returnvalue)) (Variables|Parameter|GetCheck%20Point%20Num))) (.location _returnvalue)))))
    (:then_2
      (return (LocalVariables|GetPre%20Check%20Point)))))

(fn GetBoxHeight
  ;[1 1 1] 获取需要的盒体高度
  (return (.z (- (.location (Transformation|GetSocketTransform (Variables|Default|GetWeapons) (Variables|Parameter|GetStart%20Socket%20Name) "RTS_World")) (.location (Transformation|GetSocketTransform (Variables|Default|GetWeapons) (Variables|Parameter|GetEnd%20Socket%20Name) "RTS_World"))))))

(fn GetAlreadyHitActor
  (return (Variables|Default|GetAlready%20Hit%20Actor)))

(fn GetLastHit
  (return (Variables|Default|GetLast%20Hit)))

(fn GetTraceMesh
  (return (Variables|Default|GetWeapons)))

(fn AddActortoIgnore
  (params (Add%20Actor :type Actor%20Object%20Reference%20%28by%20ref%29))
  (Utilities|Array|AddUnique (Variables|Parameter|GetActors%20to%20Ignore) Add%20Actor))

(fn RemoveActortoLgnore
  (params (Remove%20Actor :type Actor%20Object%20Reference%20%28by%20ref%29))
  (bind _returnvalue (Utilities|Array|RemoveItem (Variables|Parameter|GetActors%20to%20Ignore) Remove%20Actor))
  (return _returnvalue))

(fn GetActortoLgnore
  (return (Variables|Parameter|GetActors%20to%20Ignore)))