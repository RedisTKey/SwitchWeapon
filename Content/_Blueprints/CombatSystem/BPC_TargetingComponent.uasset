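; Actor component that gives BP_SWGASCharacter a toggleable camera lock-on for targeting.
; Enabling sphere-traces from the owner along the camera's forward vector, stores the hit actor and switches movement to face controller rotation; disabling restores the default rotation mode.
; While targeting, Tick interpolates control pitch and yaw toward the target plus a camera offset.
; TryFindTarget returns true even on a miss, so lock-on can engage without a target.
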(event Custom|Enable%20Lock%20On
  (bind (_return_value _found_target) (CallFunction|TryFindTarget))
  (if _return_value
    (CallFunction|SetTargetActor _found_target)
    (CallFunction|SetRotationMode "NewEnumerator0")
    (CallFunction|SetIsTargeting true)))

(event Custom|Disable%20Lock%20On
  (CallFunction|SetIsTargeting false)
  (CallFunction|SetRotationMode (Variables|Parameter|GetDefault%20Rotation%20Mode)))

(event Custom|Target%20Lock%20On
  (if (not (CallFunction|GetIsTargeting))
    (CallFunction|EnableLockon)
    (else
      (CallFunction|DisableLockon))))

(event EventBeginPlay
  (bind _asbp_swgascharacter (Utilities|Casting|CastToBP_SWGASCharacter (Components|GetOwner)))
  (Variables|Default|SetOwner%20Character _asbp_swgascharacter)
  (Variables|Default|SetOwner%20Controller (Pawn|GetController _asbp_swgascharacter))
  (Variables|Components|SetFollow%20Camera (Actor|GetComponentbyClass _asbp_swgascharacter "/Script/Engine.CameraComponent")))

(event EventTick
  (params (DeltaSeconds :type Float%20%28single-precision%29))
  (if (Variables|Default|GetIs%20Targeting)
    (CallFunction|UpdatingTargetControlRotation)))

(fn SetIsTargeting
  (params (enable%20Targeting :type Boolean))
  (Variables|Default|SetIs%20Targeting enable%20Targeting))

(fn GetIsTargeting
  (return (Variables|Default|GetIs%20Targeting)))

(fn TryFindTarget
  (bind _returnvalue (Components|GetOwner))
  (bind _returnvalue_2 (Transformation|GetActorLocation _returnvalue))
  (bind (_outhit _returnvalue_3) (Collision|SphereTraceForObjects _returnvalue_2 (+ (* (Math|Vector|GetForwardVector (Variables|Components|GetFollow%20Camera)) (Variables|Parameter|GetTargeting%20Distance)) _returnvalue_2) (Variables|Parameter|GetTargeting%20Radius) (Variables|Parameter|GetTarget%20Objects) false (Utilities|Array|MakeArray (Components|GetOwner)) "ForDuration"))
  (if (and _returnvalue_3 (Utilities|IsValid (.HitActor (Collision|BreakHitResult _outhit))))
    (return true (.HitActor (Collision|BreakHitResult _outhit)))
    (else
      (return true 0))))

(fn SetTargetActor
  (params (Target%20Actor :type Actor%20Object%20Reference))
  (Variables|Default|SetTarget%20Actor Target%20Actor))

(fn GetTargetActor
  (return (Variables|Default|GetTarget%20Actor)))

(fn UpdatingTargetControlRotation
  (bind _returnvalue (Utilities|Time|GetWorldDeltaSeconds))
  (bind _returnvalue_2 (Components|GetOwner))
  (bind _owner_controller (Variables|Default|GetOwner%20Controller))
  (bind _target_actor (Variables|Default|GetTarget%20Actor))
  (bind _camera_offset (Variables|Parameter|GetCamera%20Offset))
  (bind _target_rotation_interp_speed (Variables|Parameter|GetTarget%20Rotation%20Interp%20Speed))
  (bind _returnvalue_3 (Transformation|GetActorRotation _owner_controller))
  (bind _returnvalue_4 (Transformation|GetActorLocation _target_actor))
  (bind _returnvalue_5 (Transformation|GetActorLocation _returnvalue_2))
  (bind _returnvalue_6 (+ _returnvalue_4 _camera_offset))
  (bind _returnvalue_7 (Math|Rotator|FindLookatRotation _returnvalue_5 _returnvalue_6))
  (bind _returnvalue_8 (Math|Interpolation|RInterpTo _returnvalue_3 _returnvalue_7 _returnvalue _target_rotation_interp_speed))
  (if (and (Utilities|IsValid (Variables|Default|GetOwner%20Controller)) (Utilities|IsValid (Variables|Default|GetTarget%20Actor)))
    (Pawn|SetControlRotation (Variables|Default|GetOwner%20Controller) (Math|Rotator|MakeRotator (.Roll (Math|Rotator|BreakRotator _returnvalue_3)) (.pitch _returnvalue_8) (.yaw _returnvalue_8)))))

(fn SetRotationMode
  (params (New%20Rotation%20Mode :type E_RotationMode%20Enum :default "NewEnumerator0"))
  (bind _owner_character (Variables|Default|GetOwner%20Character))
  (bind _charactermovement (Variables|/Script/Engine.Character|GetCharacterMovement _owner_character))
  (bind _output_get (Variables|Default|SetCurrent%20Rotation%20Mode New%20Rotation%20Mode))
  (switch Utilities|FlowControl|Switch|SwitchonE_RotationMode _output_get
    (:NewEnumerator0
      (Variables|/Script/Engine.Pawn|SetbUseControllerRotationYaw _owner_character false)
      (Variables|/Script/Engine.CharacterMovementComponent|SetbUseControllerDesiredRotation _charactermovement true)
      (Variables|/Script/Engine.CharacterMovementComponent|SetbOrientRotationToMovement _charactermovement false))
    (:NewEnumerator1
      (Variables|/Script/Engine.Pawn|SetbUseControllerRotationYaw _owner_character false)
      (Variables|/Script/Engine.CharacterMovementComponent|SetbUseControllerDesiredRotation _charactermovement false)
      (Variables|/Script/Engine.CharacterMovementComponent|SetbOrientRotationToMovement _charactermovement true))))

(fn GetRotationMode
  (return (Variables|Default|GetCurrent%20Rotation%20Mode)))