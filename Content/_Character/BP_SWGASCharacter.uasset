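; GAS-based character Blueprint for melee combat with combos, dodges and afterimage "shadow" attacks.
; Data tables feed an ability selector gated by gameplay tags, movement state and lock-on, while movement changes update tags.
; Trace hits apply point damage plus a melee GameplayEffect to other characters of this class.
; Blank shadows spawn translucent-style stand-ins that replay a copied ability and self-destruct after its montage; tags and attributes print on tick for debugging.
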(event OnAttackHitEvent(BPC_AttackTrace)
  (params (HIt%20Result :type Hit%20Result%20Structure) (Result :type Boolean))
  (bind (_bblockinghit _binitialoverlap _time _distance _location _impactpoint _normal _impactnormal _physmat _hitactor) (Collision|BreakHitResult HIt%20Result))
  ;[0.8388 0.6038 0.008568] 测试用基础击退效果
  ; 后续封装到GAS系统里
  (Game|Damage|ApplyPointDamage _hitactor 1e+01 _impactpoint HIt%20Result)
  (bind _asbp_swgascharacter (Utilities|Casting|CastToBP_SWGASCharacter _hitactor))
  (GameplayEffects|ApplyGameplayEffectToTarget :self (Variables|Default|GetBPC_SwitchWeaponASC) :GameplayEffectClass "/Game/_GAS/GameplayEffect/GE_Melee_Damage.GE_Melee_Damage_C" :Target (Variables|BP_SWGASCharacter_C|GetBPC_SwitchWeaponASC _asbp_swgascharacter)))

(event Custom|Try%20Activate%20Copyed%20Ability
  ;[0.05098 0.05098 0.05098] 残影攻击
  (bind _shadow_ability_info (Variables|Shadow|GetShadow%20Ability%20Info)
    (:then
      (bind _output_get (Variables|Combat|SetExcuted%20Ability%20Info (Utilities|Struct|MakeS_SingleAbilityInfo (.Gameplay%20Ability (Default|GetInfo _shadow_ability_info)) (.AnimMontage (Default|GetInfo _shadow_ability_info)) "(TagName=\"\")" "(TagName=\"\")" "(TagName=\"\")")))
      (Abilities|TryActivateAbilitybyClass (Variables|Default|GetBPC_SwitchWeaponASC) (.Ability (Utilities|Struct|BreakS_SingleAbilityInfo _output_get)) true)
      (Utilities|FlowControl|Delay (Variables|/Script/Engine.AnimSequenceBase|GetSequenceLength (.AnimMontage (Utilities|Struct|BreakS_SingleAbilityInfo _output_get))))
      (Actor|DestroyActor))
    (:else)))

(event Custom|Spawn%20From%20Blank%20Shadow
  ;[0.05098 0.05098 0.05098] 作为白板残影，放置角色
  (if (Variables|Shadow|GetbIsBlankShadow)
    (bind _shadow_ability_info (Variables|Shadow|GetShadow%20Ability%20Info)
      (:then
        (bind _returnvalue (Game|SpawnActorfromClass (Utilities|GetClass (.Actor (Default|GetInfo _shadow_ability_info))) (Math|Transform|MakeTransform (Transformation|GetActorLocation) (Transformation|GetActorRotation) "1.000000,1.000000,1.000000") "AlwaysSpawn" "MultiplyWithRoot" 0 0))
        (CallFunction|SpawnedasShadow _returnvalue)
        (Ability|GameplayEffect|AddLooseGameplayTags _returnvalue (GameplayTags|MakeGameplayTagContainerfromTag "(TagName=\"State.CantBeHit\")"))
        (Actor|DestroyActor))
      (:else))))

(event Custom|Spawned%20As%20Shadow
  ;[0.05098 0.05098 0.05098] 残影技能配置
  (Utilities|FlowControl|Sequence
    (:then_2
      (CallFunction|TryActivateCopyedAbility))))

(event EventOnMovementModeChanged
  (params (PrevMovementMode :type EMovementMode%20Enum :default "MOVE_None") (NewMovementMode :type EMovementMode%20Enum :default "MOVE_None") (PrevCustomMode :type Byte :default 0) (NewCustomMode :type Byte :default 0))
  ;[0.05098 0.05098 0.05098] 用于通知其他蓝图（如动画蓝图，移动状态改变）
  (Default|CallOnMovementModeChanged NewMovementMode)
  (switch Utilities|FlowControl|Switch|SwitchonEMovementMode NewMovementMode
    (:MOVE_Walking
      (GameplayTag|SwitchMovementTag "(TagName=\"Movement.Walk\")"))
    (:MOVE_NavWalking
      (GameplayTag|SwitchMovementTag "(TagName=\"Movement.NavWalk\")"))
    (:MOVE_Falling
      (GameplayTag|SwitchMovementTag "(TagName=\"Movement.Fly\")"))
    (:MOVE_Swimming
      (GameplayTag|SwitchMovementTag "(TagName=\"Movement.Swim\")"))
    (:MOVE_Flying
      (GameplayTag|SwitchMovementTag "(TagName=\"Movement.Fly\")"))
    (:MOVE_Custom
      (GameplayTag|SwitchMovementTag "(TagName=\"Movement.Custom\")"))))

(event EventBeginPlay
  (Utilities|FlowControl|Sequence
    (:then_0
      ;[1 1 1] 用于初始化作为shadow的配置，正常生成的角色不用管
      (Shadow|InitShadowSetting))
    (:then_1
      (GameplayAbility|InitAbilities)
      (CallFunction|BindASCRelatedEvent))))

(event EventTick
  (params (DeltaSeconds :type Float%20%28single-precision%29))
  (DebugTools|PrintInfo (Variables|DebugVar|GetPrint%20to%20INFO%20Screen)))

(event Game|Damage|EventAnyDamage
  (params (Damage :type Float%20%28single-precision%29) (DamageType :type Damage%20Type%20Object%20Reference) (InstigatedBy :type Controller%20Object%20Reference) (DamageCauser :type Actor%20Object%20Reference))
  ;[0.8388 0.6038 0.008568] 测试用基础击退效果
  ; 后续封装到GAS系统里
)

(fn ConstructionScript)

(fn PrintInfo
  (params (bShouldPrint? :type Boolean))
  (bind _bpc_switchweaponasc (Variables|Default|GetBPC_SwitchWeaponASC))
  (if bShouldPrint?
    (Utilities|FlowControl|Sequence
      (:then_0
        (Utilities|Array|Clear (LocalVariables|GetPrint%20Message)))
      (:then_1
        ;[0.05098 0.05098 0.05098] 角色名字
        (Utilities|Array|Add (LocalVariables|GetPrint%20Message) (Utilities|GetDisplayName self)))
      (:then_2
        ;[0.05 0.05 0.05] 输出角色所有的Tag
        (LocalVariables|SetTemp%20Record " Tag: ")
        (for _array_element (.gameplaytags (GameplayTags|GetOwnedGameplayTags _bpc_switchweaponasc :!class /Script/GameplayTags.GameplayTagAssetInterface))
          (LocalVariables|SetTemp%20Record (Utilities|String|Append (LocalVariables|GetTemp%20Record) "&" (Utilities|String|ToString(Name) (GameplayTags|GetTagName _array_element)))))
        (Utilities|Array|Add (LocalVariables|GetPrint%20Message) (LocalVariables|GetTemp%20Record)))
      (:then_3
        ;[0.05098 0.05098 0.05098] 输出角色的所有Attribute
        (LocalVariables|SetTemp%20Record "")
        (for _array_element_2 (Class|AbilitySystemComponent|GetAllAttributes (Variables|Default|GetBPC_SwitchWeaponASC))
          (LocalVariables|SetTemp%20Record (Utilities|String|Append (LocalVariables|GetTemp%20Record) (Utilities|Struct|BreakGameplayAttribute _array_element_2) ":" (Utilities|String|ToString(Float) (.ReturnValue (Ability|Attribute|GetFloatAttributefromAbilitySystemComponent _bpc_switchweaponasc _array_element_2))) "&")))
        (Utilities|Array|Add (LocalVariables|GetPrint%20Message) (LocalVariables|GetTemp%20Record)))
      (:then_4
        ;[0.05098 0.05098 0.05098] 输出所有信息
        (for _array_element_3 (LocalVariables|GetPrint%20Message)
          (Development|PrintString _array_element_3 true true "(R=0.039546,G=0.651406,B=0.000000,A=1.000000)" (Utilities|Time|GetWorldDeltaSeconds)))))))

(fn OnTagChanged
  (params (Tag :type Gameplay%20Tag%20Structure%20%28by%20ref%29) (TagExists :type Boolean))
  ;[1 1 1] Tag Changed的回调函数，主要是用来做第二层的触发GA判定
)

(fn OnAbilityEnded
  (params (AbilityReference :type Gameplay%20Ability%20Object%20Reference) (wasCancelled :type Boolean)))

(fn OnGameplayAttributeChanged
  (params (Attribute :type Gameplay%20Attribute%20Structure) (Value :type Float%20%28single-precision%29)))

(fn SwitchMovementTag
  (params (New%20Movement%20Mode%20Tag :type Gameplay%20Tag%20Structure))
  (bind _self self)
  ;[1 1 1] 切换用于标识移动状态的Tag
  (Ability|GameplayEffect|RemoveLooseGameplayTags _self (GameplayTags|MakeLiteralGameplayTagContainer "(GameplayTags=((TagName=\"Movement.Custom\"),(TagName=\"Movement.Fall\"),(TagName=\"Movement.Fly\"),(TagName=\"Movement.NavWalk\"),(TagName=\"Movement.Walk\"),(TagName=\"Movement.Swim\")))"))
  (Ability|GameplayEffect|AddLooseGameplayTags _self (GameplayTags|MakeGameplayTagContainerfromTag New%20Movement%20Mode%20Tag)))

(fn TryFindExcuteComboAbility
  (params (InputAction%20Tag :type Gameplay%20Tag%20Structure))
  (bind _charactermovement (Variables|Character|GetCharacterMovement))
  (bind _charactermovement_2 (Variables|Character|GetCharacterMovement))
  (|SwitchGameplayTag InputAction%20Tag
    (:InputAction.Melee
      (for _array_element (Variables|Combat|GetCombo%20Data)
        (if (== (.TriggerInputActionTag (Utilities|Struct|BreakS_SingleAbilityInfo _array_element)) InputAction%20Tag)
          (LocalVariables|SetCombo%20Tag (.ComboTag (Utilities|Struct|BreakS_SingleAbilityInfo _array_element)))
          (if (Math|Boolean|ANDBoolean (or (== (LocalVariables|GetCombo%20Tag) "(TagName=\"Combo.Ground1\")") (GameplayTags|HasMatchingGameplayTag (Variables|Default|GetBPC_SwitchWeaponASC) (LocalVariables|GetCombo%20Tag))) (or (and (== (LocalVariables|GetCombo%20Tag) "(TagName=\"Combo.Ground1\")") (not (GameplayTags|HasMatchingGameplayTag (Variables|Default|GetBPC_SwitchWeaponASC) "(TagName=\"State.Attacking\")"))) (and (!= (LocalVariables|GetCombo%20Tag) "(TagName=\"Combo.Ground1\")") (GameplayTags|HasMatchingGameplayTag (Variables|Default|GetBPC_SwitchWeaponASC) "(TagName=\"State.Attacking\")"))) (and (not (AI|Components|NavMovement|IsFalling _charactermovement)) (not (Class|NavMovementComponent|IsFlying _charactermovement))))
            (return _array_element true))))
      (return "" false))
    (:InputAction.Dodge
      (Utilities|FlowControl|Sequence
        (:then_0
          (LocalVariables|SetbCanDodge (and (not (Class|NavMovementComponent|IsFlying _charactermovement_2)) (not (AI|Components|NavMovement|IsFalling _charactermovement_2))))
          (LocalVariables|SetbHasDodgeDir (GameplayTags|HasMatchingGameplayTag (Variables|Default|GetBPC_SwitchWeaponASC) "(TagName=\"InputAction.DodgeDir\")"))
          (LocalVariables|SetbIsTargeting (Default|GetIsTargeting (Variables|Default|GetBPC_CameraSystem))))
        (:then_1
          (if (and (LocalVariables|GetbCanDodge) (LocalVariables|GetbIsTargeting))
            (if (LocalVariables|GetbHasDodgeDir)
              (for _array_element_2 (Variables|Dodge|GetDodge%20Data)
                (if (GameplayTags|HasMatchingGameplayTag (Variables|Default|GetBPC_SwitchWeaponASC) (.DodgeDirecitonTag (Utilities|Struct|BreakS_SingleAbilityInfo _array_element_2)))
                  (return _array_element_2 true)))
              (return "" false)
              (else
                ;[1 1 1] 锁定+无朝向
                (if true
                  (return (Variables|Dodge|GetBackward%20Dodge%20Data) true))))
            (elif (and (LocalVariables|GetbCanDodge) (not (LocalVariables|GetbIsTargeting)))
              (if (LocalVariables|GetbHasDodgeDir)
                (return (Variables|Dodge|GetForward%20Dodge%20Data) true)
                (elif true
                  (return (Variables|Dodge|GetBackward%20Dodge%20Data) true))))))))))

(fn ResetCombo
  (params (TagContainer :type Gameplay%20Tag%20Container%20Structure%20%28by%20ref%29))
  ;[0.05098 0.05098 0.05098] 删除原有的所有Combo Tag
  (Utilities|FlowControl|Sequence
    (:then_0
      (if (GameplayTags|HasAnyTags (GameplayTags|GetOwnedGameplayTags (Variables|Default|GetBPC_SwitchWeaponASC) :!class /Script/GameplayTags.GameplayTagAssetInterface) (GameplayTags|MakeLiteralGameplayTagContainer "(GameplayTags=((TagName=\"Combo\")))"))
        (Ability|GameplayEffect|RemoveLooseGameplayTags self (GameplayTags|MakeLiteralGameplayTagContainer "(GameplayTags=((TagName=\"Combo.Ground1\"),(TagName=\"Combo.Ground2\"),(TagName=\"Combo.Ground3\"),(TagName=\"Combo.Ground4\")))"))))
    (:then_1
      ;[0.05098 0.05098 0.05098] 添加新标签
      (Ability|GameplayEffect|AddLooseGameplayTags self TagContainer))))

(fn InitAbilities
  (bind _combo_data_table (Variables|Combat|GetCombo%20Data%20Table))
  (Utilities|FlowControl|Sequence
    (:then_0
      ;[1 1 1] 读取技能表格
      (bind _outrownames (DataTable|GetDataTableRowNames _combo_data_table))
      (for _array_element _outrownames
        (bind _returnvalue (Utilities|GetDataTableRow _combo_data_table _array_element)
          (:then
            (Utilities|Array|Add (Variables|Combat|GetCombo%20Data) _returnvalue)))))
    (:then_1
      ;[1 1 1] 读取翻滚表格
      (bind _dodge_data_table (Variables|Dodge|GetDodge%20Data%20Table)
        (:then
          (bind _outrownames_2 (DataTable|GetDataTableRowNames _dodge_data_table))
          (for _array_element_2 _outrownames_2
            (bind _returnvalue_2 (Utilities|GetDataTableRow _dodge_data_table _array_element_2)
              (:then
                (Utilities|Array|Add (Variables|Dodge|GetDodge%20Data) _returnvalue_2)
                (|SwitchGameplayTag (.DodgeDirecitonTag (Utilities|Struct|BreakS_SingleAbilityInfo _returnvalue_2))
                  (:InputAction.DodgeDir.F
                    (Variables|Dodge|SetForward%20Dodge%20Data _returnvalue_2))
                  (:InputAction.DodgeDir.B
                    (Variables|Dodge|SetBackward%20Dodge%20Data _returnvalue_2)))))))
        (:else)))
    (:then_2
      (return))))

(fn BindASCRelatedEvent
  (bind _bpc_switchweaponasc (Variables|Default|GetBPC_SwitchWeaponASC))
  (EventDispatchers|BindEventtoOnTagUpdatedDelegate _bpc_switchweaponasc (EventDispatchers|CreateEvent :!event OnTagChanged))
  (EventDispatchers|BindEventtoOnAbilityEndedBlueprintCallable _bpc_switchweaponasc (EventDispatchers|CreateEvent :!event OnAbilityEnded))
  (EventDispatchers|BindEventtoOnGameplayAttributeChanged _bpc_switchweaponasc (EventDispatchers|CreateEvent :!event OnGameplayAttributeChanged)))

(fn InitShadowSetting
  (bind _self self)
  (bind _returnvalue (AI|GetAIController _self))
  (if (Variables|Default|GetbIsShadow)
    (Utilities|FlowControl|Sequence
      (:then_0
        ;[0.05098 0.05098 0.05098] 初始化残影基本配置
        (Collision|SetCollisionEnabled (Variables|Default|GetCapsuleComponent) "NoCollision")
        (Pawn|Components|CharacterMovement|SetMovementMode (Variables|Character|GetCharacterMovement) "MOVE_Flying" 0)
        (Utilities|FlowControl|Sequence
          (:then_0
            (Utilities|IsValid _returnvalue
              (:Is%20Valid
                (Pawn|UnPossess _returnvalue))))))
      (:then_1
        ;[0.05098 0.05098 0.05098] 配置残影材质
        (Rendering|Material|SetMaterial (Variables|Character|GetMesh) 0 "/Game/HologramVFX/Material/Hologram/M_PlanetRing.M_PlanetRing")
        (for _array_element (Components|GetChildrenComponents (Variables|Character|GetMesh) false)
          (bind _asprimitive_component (Utilities|Casting|CastToPrimitiveComponent _array_element))
          (Rendering|Material|SetMaterial _asprimitive_component 0 "/Game/HologramVFX/Material/Hologram/M_PlanetRing.M_PlanetRing"))))
    (else
      (return))))